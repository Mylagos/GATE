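; Purple-room puzzle cube that mirrors its linked BlueCube when the player swaps between rooms.
; On room-change events, a flag alternates between copying BlueCube's transform (shifted by a fixed Y offset) and velocities with physics on, and freezing physics after a short delay.
; The button's grab event permanently stops syncing so later swaps only disable physics, avoiding collision problems, and its press event turns the cube's material blue.
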(event `self.ReceiveBeginPlay`
  (bind _button (`self.Button`))
  (add `/Game/GATE_CPP/Blueprints/Puzzle_Actors/PurpleRoom_PuzzleButton.SwitchPressedPurple` _button (delegate `ChangeCubeColor`))
  (add `/Game/GATE_CPP/Blueprints/FirstPersonCharacter.ChangeRoom` (`self.Player`) (delegate `CubeSync`))
  (add `/Game/GATE_CPP/Blueprints/Puzzle_Actors/PurpleRoom_PuzzleButton.Cube GrabbedPurple` _button (delegate `StopSyncCube`)))

(event `StopSyncCube`
  (set `self.Is on Button` true))

(event `ChangeCubeColor`
  (params (Switch :type "/Game/GATE_CPP/Blueprints/Puzzle_Actors/PurpleRoom_PuzzleButton Object Reference"))
  (if (== Switch (`self.Button`))
    (`PrimitiveComponent.SetMaterial` (`self.Cube`) 1 "/Game/GATE/Textures/Emissive_Material/EBlue.EBlue")))

(event `CubeSync`
  (bind _cube (`self.Cube`))
  (bind _cube_2 (`/Game/GATE_CPP/Blueprints/Puzzle_Actors/BlueRoom_PuzzleCube.Cube` (`self.BlueCube`)))
  (if (`self.Is On Button`)
    (`PrimitiveComponent.SetSimulatePhysics` (`self.Cube`) false)
    (elif (`self.Swap To Purple Room`)
      (`PrimitiveComponent.SetSimulatePhysics` _cube true)
      (`|ExecutionSequence`
        (:`then_0`
          ;[1 1 1] Setting all the values
          (`SceneComponent.K2_SetWorldLocation` _cube (+ (`SceneComponent.K2_GetComponentLocation` _cube_2) (0.0 30000.0 0.0)) false false))
        (:`then_1`
          (`SceneComponent.K2_SetWorldRotation` _cube (`SceneComponent.K2_GetComponentRotation` _cube_2) false false))
        (:`then_2`
          ;[1 1 1] Getting all the values we need for the sync
          (bind _returnvalue (`PrimitiveComponent.GetPhysicsLinearVelocity` _cube_2 "None"))
          (`PrimitiveComponent.SetPhysicsLinearVelocity` _cube _returnvalue false "None"))
        (:`then_3`
          (`PrimitiveComponent.SetPhysicsAngularVelocityInDegrees` _cube (`PrimitiveComponent.GetPhysicsAngularVelocityInDegrees` _cube_2 "None") false "None"))
        (:`then_4`
          (set `self.Swap To Purple Room` false)))
      (else
        (`KismetSystemLibrary.Delay` 0.01)
        (`PrimitiveComponent.SetSimulatePhysics` _cube false)
        (set `self.Swap To Purple Room` true)))))

(event `self.ReceiveTick`
  (params (DeltaSeconds :type "Float (single-precision)")))

(fn `UserConstructionScript`)
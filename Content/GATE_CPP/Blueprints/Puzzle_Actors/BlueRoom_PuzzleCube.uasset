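; Blue room puzzle cube that stays in sync with its purple room counterpart when the player changes rooms.
; When its linked Button reports being pressed, it applies the green material and flags itself as on the button.
; On room change it freezes physics if on the button; otherwise, depending on SwapToPurpleRoom, it either re-enables physics or also copies PurpleCube's offset location, rotation and velocities.
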(event `self.ReceiveBeginPlay`
  (add `/Game/GATE_CPP/Blueprints/Puzzle_Actors/BlueRoom_PuzzleButton.SwitchPressed` (`self.Button`) (delegate `ChangeCubeColor`))
  (add `/Game/GATE_CPP/Blueprints/FirstPersonCharacter.ChangeRoom` (`self.Player`) (delegate `CustomEvent`)))

(event `ChangeCubeColor`
  (params (NewParam :type "/Game/GATE_CPP/Blueprints/Puzzle_Actors/BlueRoom_PuzzleButton Object Reference"))
  (if (== (`self.Button`) NewParam)
    (`PrimitiveComponent.SetMaterial` (`self.Cube`) 1 "/Game/GATE/Textures/Emissive_Material/EGreen.EGreen")
    (set `self.Is on Button` true)))

(event `self.ReceiveTick`
  (params (DeltaSeconds :type "Float (single-precision)")))

(event `CustomEvent`
  (bind _cube (`self.Cube`))
  (bind _cube_2 (`/Game/GATE_CPP/Blueprints/Puzzle_Actors/PurpleRoom_PuzzleCube.Cube` (`self.PurpleCube`)))
  (if (`self.Is On Button`)
    (`PrimitiveComponent.SetSimulatePhysics` (`self.Cube`) false)
    (elif (`self.Swap To Purple Room`)
      (`KismetSystemLibrary.Delay` 0.01)
      (`PrimitiveComponent.SetSimulatePhysics` _cube true)
      (set `self.Swap To Purple Room` true)
      (else
        (`PrimitiveComponent.SetSimulatePhysics` _cube true)
        (`|ExecutionSequence`
          (:`then_0`
            ;[1 1 1] Setting all the values
            (`SceneComponent.K2_SetWorldLocation` _cube (+ (`SceneComponent.K2_GetComponentLocation` _cube_2) (0.0 -30000.0 0.0)) false false))
          (:`then_1`
            (`SceneComponent.K2_SetWorldRotation` _cube (`SceneComponent.K2_GetComponentRotation` _cube_2) false false))
          (:`then_2`
            ;[1 1 1] Getting all the values we need for the sync
            (bind _returnvalue (`PrimitiveComponent.GetPhysicsLinearVelocity` _cube_2 "None"))
            (`PrimitiveComponent.SetPhysicsLinearVelocity` _cube _returnvalue false "None"))
          (:`then_3`
            (`PrimitiveComponent.SetPhysicsAngularVelocityInDegrees` _cube (`PrimitiveComponent.GetPhysicsAngularVelocityInDegrees` _cube_2 "None") false "None"))
          (:`then_4`
            (set `self.Swap To Purple Room` false)))))))

(fn `UserConstructionScript`)
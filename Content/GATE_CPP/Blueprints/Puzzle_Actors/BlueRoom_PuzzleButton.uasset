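; Blue Room puzzle button actor that captures a BlueRoom_PuzzleCube, draws it into itself and signals that it is pressed.
; The grabber trigger disables the cube's physics and grabs it, then Tick starts a timeline lerping it horizontally toward the button base while rotating it.
; A second timeline then pushes it inside, lerping all three axes.
; A separate button trigger fires the SwitchPressed dispatcher and turns the lights green when the cube overlaps it.
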(event `self.TriggerItemGrabber.OnComponentBeginOverlap`
  (params (OverlappedComponent :type "PrimitiveComponent Object Reference") (OtherActor :type "Actor Object Reference") (OtherComp :type "PrimitiveComponent Object Reference") (OtherBodyIndex :type Integer) (bFromSweep :type Boolean) (SweepResult :type "HitResult Structure (by ref)"))
  ;[1 1 1] Setup Cube Grab
  (if (== (`GameplayStatics.GetObjectClass` OtherActor) "/Game/GATE_CPP/Blueprints/Puzzle_Actors/BlueRoom_PuzzleCube.BlueRoom_PuzzleCube_C")
    (bind _output_get (set `self.Cube` OtherComp))
    (`PrimitiveComponent.SetSimulatePhysics` _output_get false)
    (`PhysicsHandleComponent.GrabComponentAtLocation` (`self.PhysicsHandle`) _output_get "None" (`SceneComponent.K2_GetComponentLocation` _output_get))
    (set `self.IsGrabbing` true)))

(event `self.ReceiveTick`
  (params (DeltaSeconds :type "Float (single-precision)"))
  (bind _cube (`self.Cube`))
  (bind _returnvalue (`SceneComponent.K2_GetComponentRotation` _cube))
  (bind _returnvalue_2 (`SceneComponent.K2_GetComponentLocation` _cube))
  (bind _returnvalue_3 (+ (* (- _returnvalue_2 (`SceneComponent.K2_GetComponentLocation` (`self.Basic`))) -2.0) _returnvalue_2))
  ;[1 1 1] Cube "Animation"
  (if (`self.IsGrabbing`)
    (bind (_direction _newtrack_0) (`Timeline|Timeline_0`)
      (:`Update`
        (`SceneComponent.K2_SetWorldLocationAndRotation` _cube (`KismetMathLibrary.MakeVector` (.x (`KismetMathLibrary.VLerp` _returnvalue_2 _returnvalue_3 _newtrack_0)) (.y (`KismetMathLibrary.VLerp` _returnvalue_2 _returnvalue_3 _newtrack_0)) (.z _returnvalue_2)) (`KismetMathLibrary.RLerp` _returnvalue (* _returnvalue -1.0) _newtrack_0) false false))
      (:`Finished`
        ;;[1 1 1] Delayed lerp to push the cube inside
        (bind (_direction_2 _newtrack_0_2) (`Timeline|Timeline_1`)
          (:`Update`
            (`SceneComponent.K2_SetWorldLocation` _cube (`KismetMathLibrary.VLerp` _returnvalue_2 _returnvalue_3 _newtrack_0_2) false false)))))))

(event `self.TriggerButton.OnComponentBeginOverlap`
  (params (OverlappedComponent :type "PrimitiveComponent Object Reference") (OtherActor :type "Actor Object Reference") (OtherComp :type "PrimitiveComponent Object Reference") (OtherBodyIndex :type Integer) (bFromSweep :type Boolean) (SweepResult :type "HitResult Structure (by ref)"))
  (bind _lights (`self.Lights`))
  ;[1 1 1] ActivateEventDispatcher
  (if (== (`GameplayStatics.GetObjectClass` OtherActor) "/Game/GATE_CPP/Blueprints/Puzzle_Actors/BlueRoom_PuzzleCube.BlueRoom_PuzzleCube_C")
    (`self.SwitchPressed` self)
    (bind _output_get (set `self.IsActivated` true))
    (if _output_get
      (`PrimitiveComponent.SetMaterial` _lights 0 "/Game/GATE/Textures/Emissive_Material/EGreen.EGreen")
      (else
        (`PrimitiveComponent.SetMaterial` _lights 0 "/Game/GATE/Textures/Emissive_Material/EOrange.EOrange")))))

(fn `UserConstructionScript`)
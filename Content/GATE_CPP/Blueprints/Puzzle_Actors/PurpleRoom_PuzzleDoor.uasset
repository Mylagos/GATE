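; Puzzle door for the purple room that unlocks when its linked button's purple switch is pressed.
; On BeginPlay it binds to that button's event, and the handler confirms the switch matches before clearing the lock.
; Unlocking turns the frame and door blue, then after a short delay a timeline lerps the door's relative location downward.
; The construction script's lock-based door coloring is disconnected and never runs.
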(event `self.ReceiveBeginPlay`
  (add `/Game/GATE_CPP/Blueprints/Puzzle_Actors/PurpleRoom_PuzzleButton.SwitchPressedPurple` (`self.Button`) (delegate `Unlock Door`)))

(event `Unlock Door`
  (params (Switch :type "/Game/GATE_CPP/Blueprints/Puzzle_Actors/PurpleRoom_PuzzleButton Object Reference"))
  (bind _door_frame (`self.Door_Frame`))
  (bind _door (`self.Door`))
  (if (== (`self.Button`) Switch)
    (bind _output_get (set `self.IsLocked` false))
    (if _output_get
      (`PrimitiveComponent.SetMaterial` _door_frame 1 "/Game/GATE/Textures/Emissive_Material/EPurple.EPurple")
      (else
        (`PrimitiveComponent.SetMaterial` _door_frame 1 "/Game/GATE/Textures/Emissive_Material/EBlue.EBlue")
        (`PrimitiveComponent.SetMaterial` _door 0 "/Game/GATE/Textures/Emissive_Material/EBlue.EBlue")
        (`KismetSystemLibrary.Delay` 1.0)
        (bind (_direction _newtrack_0) (`Timeline|Timeline_0`)
          (:`Update`
            (`SceneComponent.K2_SetRelativeLocation` _door (`KismetMathLibrary.VLerp` (0.0 0.0 200.0) (0.0 0.0 -750.0) _newtrack_0) false false)))))))

(fn `UserConstructionScript`)